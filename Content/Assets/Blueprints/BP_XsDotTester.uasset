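; BP_XsDotTester is a test actor for Xsens DOT sensors, binding Bluetooth devices to its joint scene components.
; On BeginPlay it registers XsBindingManager with XsensDotManager's XsDot and subscribes to button-click events, whose handler is empty.
; It then loops over BindingTagAndDeviceAddress, binding each tag and device address to Joint0, Joint1 or Joint2 by array index as an enabled, local binding.
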(event `self.ReceiveBeginPlay`
  (bind _xsdot (`/Game/Assets/Blueprints/BP_XsensDotManager.XsDot` (`self.XsensDotManager`)))
  (add `XsDot.OnButtonClicked` _xsdot (delegate `커스텀이벤트`))
  (`XsDot.AddBindingManager` _xsdot (`self.XsBindingManager`))
  (for (_array_element _array_index) (`self.BindingTagAndDeviceAddress`)
    (bind (_tag _devicebluetoothaddress) (break `/Game/Assets/Blueprints/Struct/BindingMinimalInfo` _array_element))
    (`XsBindingManager.Bind` (`self.XsBindingManager`) _tag (make `XsBindingInfo` (`|GetArrayItem` (`|MakeArray` (`self.Joint0`) (`self.Joint1`) (`self.Joint2`)) _array_index) _devicebluetoothaddress true true) false)))

(event `커스텀이벤트`
  (params (deviceAddress :type String) (timestamp :type Integer)))

(event `self.ReceiveTick`
  (params (DeltaSeconds :type "Float (single-precision)")))

(fn `UserConstructionScript`)