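; BP_People is a person actor whose skeletal mesh uses a Control Rig to look at a target actor.
; On BeginPlay the target defaults to player 0's pawn if none is valid.
; The ControlRig component maps the whole mesh on pre-initialize, then before each forwards solve passes the target's location and the IsLooking flag into CR_People.
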(event `self.ReceiveBeginPlay`
  (`/Engine/EditorBlueprintResources/StandardMacros.IsValid` (`self.LookingTarget`)
    (:`Is Not Valid`
      (set `self.LookingTarget` (`GameplayStatics.GetPlayerPawn` 0)))))

(event `self.ControlRig.OnPreInitializeDelegate`
  (params (Component :type "ControlRigComponent Object Reference"))
  (`ControlRigComponent.AddMappedCompleteSkeletalMesh` Component (`self.Mesh`)))

(event `self.ControlRig.OnPreForwardsSolveDelegate`
  (params (Component :type "ControlRigComponent Object Reference"))
  (bind _lookingtarget (`self.LookingTarget`))
  (`/Engine/EditorBlueprintResources/StandardMacros.IsValid` _lookingtarget
    (:`Is Valid`
      (bind _ascr_people (cast `/Game/Assets/Mesh/CR_People` (`ControlRigComponent.GetControlRig` Component)))
      (set `/Game/Assets/Mesh/CR_People.LookAtLocation` (`self.K2_GetActorLocation` _lookingtarget) _ascr_people)
      (set `/Game/Assets/Mesh/CR_People.isLooking` (`self.isLooking`) _ascr_people))))

(fn `UserConstructionScript`)