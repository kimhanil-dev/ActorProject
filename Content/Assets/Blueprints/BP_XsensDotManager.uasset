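; Manager actor for Xsens DOT motion sensors that handles Bluetooth scanning, connection and live orientation data.
; Scanning starts at BeginPlay, listing detected devices in a WB_Debug widget, and connection requests report results back to their requester.
; Connected devices are stored in a map, polled every Tick for quaternions that are broadcast through OnDataUpdated.
; SetRotationZero or the Q key resets sensor orientation, and scanning stops at EndPlay.
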(event `self.ReceiveBeginPlay`
  (bind _returnvalue (`GameplayStatics.GetPlayerController` 0))
  (`self.EnableInput` _returnvalue)
  ;[1 1 1] Start Scanning
  (`XsDot.StartScanning` (`self.XsDot`) (delegate `OnDeviceDetected`))
  ;[1 1 1] Debug Widget Init
  (bind _returnvalue_2 (`|CreateWidget` "/Game/Assets/Blueprints/UMG/WB_Debug.WB_Debug_C" _returnvalue))
  (bind _output_get (set `self.DebugWidget` _returnvalue_2))
  (`/Game/Assets/Blueprints/UMG/WB_Debug.Init` _output_get self)
  (`UserWidget.AddToViewport` _output_get 0))

(event `OnDeviceDetected`
  (params (deviceAddress :type String))
  ;[1 1 1] On Device Detected
  (`KismetArrayLibrary.Array_Add` (`self.DetectedDevices`) deviceAddress)
  (`/Game/Assets/Blueprints/UMG/WB_Debug.AddDevice` (`self.DebugWidget`) deviceAddress))

(event `self.ReceiveTick`
  (params (DeltaSeconds :type "Float (single-precision)"))
  ;[1 0.7651 0] Receive Rotation Value And Update Rotations
  (bind _keys (`BlueprintMapLibrary.Map_Keys` (`self.DeviceInfo`)))
  (for _array_element _keys
    (bind (_rotation _acceleration _quat _valid) (`XsDot.GetLiveData` (`self.XsDot`) _array_element))
    (if _valid
      (`BlueprintMapLibrary.Map_Add` (`self.DeviceInfo`) _array_element _quat)
      (`self.OnDataUpdated` _quat))))

(event `self.ReceiveEndPlay`
  (params (EndPlayReason :type "EEndPlayReason Enum" :default "Destroyed"))
  ;[0.5694 0.5848 1] Stop Scanning
  (`XsDot.StopScanning` (`self.XsDot`)))

(event `/Game/Assets/Blueprints/UMG/BPI_Connector.RequestDeviceConnection`
  (params (DeviceAddress :type String) (Requester :type "/Game/Assets/Blueprints/UMG/BPI_ConnectionRequester Interface"))
  ;[0 0.2456 1 1 34] Deviec Connection Sequences
  (set `self.ConnectionRequester` Requester)
  (bind _devicenotfound (`XsDot.ConnectDevice` (`self.XsDot`) DeviceAddress (delegate `OnDeviceConnectionResult`)))
  (if _devicenotfound
    (`/Game/Assets/Blueprints/UMG/BPI_ConnectionRequester.OnConnectionRequestFaild` (`self.ConnectionRequester`) "device not found")))

(event `OnDeviceConnectionResult`
  (params (deviceAddress :type String) (isSuccess :type Boolean))
  ;[0 0.2456 1 1 34] Deviec Connection Sequences
  (`/Game/Assets/Blueprints/UMG/BPI_ConnectionRequester.OnConnectResult` (`self.ConnectionRequester`) deviceAddress isSuccess)
  (if isSuccess
    (`XsDot.SetLiveDataOutputRate` (`self.XsDot`) (enumliteral `EOutputRate` "OR_30HZ"))
    (`BlueprintMapLibrary.Map_Add` (`self.DeviceInfo`) deviceAddress)
    (`self.OnDeviceConnected` deviceAddress)))

(event `SetRotationZero`
  (params (deviceBluetoothAddress :type String))
  ;[0 1 0.7971] Reset XsDot Orientation
  (`XsDot.ResetOrientation` (`self.XsDot`) :!label _label))

(event `Key|Q`
  (params (Key :type "Key Structure"))
  ;[0 1 0.7971] Reset XsDot Orientation
  (:`Pressed`
    (goto _label)))

(fn `CheckVelocityThreshold`
  (params (Vector :type "Vector Structure"))
  (returns (ok :type Boolean))
  (bind _returnvalue (>= (`KismetMathLibrary.VSize` Vector) 0.0))
  (if _returnvalue
    (return _returnvalue)))

(fn `UserConstructionScript`)