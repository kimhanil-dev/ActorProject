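; BP_SequenceManager is an input-driven actor that steps through an array of level sequences and can hide a screen actor.
; It enables player input on BeginPlay, and the E debug key or P plays the sequence at the current index, then increments that index.
; The O key hides the Screen actor in game.
; The index has no bounds check or wraparound.
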(event Custom|PlayNextSequence
  (bind _result (Math|Integer|IncrementInt (Variables|Default|GetCurrentSequence))
    (:%20%20
      (Sequencer|Player|Play (Variables|/Script/LevelSequence.LevelSequenceActor|GetSequencePlayer (Utilities|Array|Get(acopy) (Variables|Default|GetSequences) _result)) :!class /Script/MovieScene.MovieSceneSequencePlayer))))

(event Custom|HideScreen
  (Rendering|SetActorHiddenInGame (Variables|Default|GetScreen) true))

(event EventBeginPlay
  (Input|EnableInput (Game|GetPlayerController 0)))

(event Input|KeyboardEvents|DebugKeyE
  (params (Key :type Key%20Structure :default "None") (ActionValue :type Input%20Action%20Value%20Structure))
  (:Pressed
    (CallFunction|PlayNextSequence)))

(event Input|KeyboardEvents|P
  (params (Key :type Key%20Structure :default "None"))
  (:Pressed
    (CallFunction|PlayNextSequence)))

(event Input|KeyboardEvents|O
  (params (Key :type Key%20Structure :default "None"))
  (:Pressed
    (CallFunction|HideScreen)))

(fn ConstructionScript)