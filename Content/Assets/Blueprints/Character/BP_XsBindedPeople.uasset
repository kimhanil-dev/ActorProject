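; BP_XsBindedPeople is an actor whose skeletal arm is driven by Xsens DOT motion sensors.
; On BeginPlay it registers its binding manager with the DOT manager and anonymously binds configured Bluetooth device addresses to three scene components.
; Before each Control Rig forward solve, it copies those components' relative rotations as quaternions into CR_XsBinded's shoulder, forearm and hand rotations.
; The button-click handler is bound but empty.
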(event `self.ReceiveBeginPlay`
  (bind _xsdot (`/Game/Assets/Blueprints/BP_XsensDotManager.XsDot` (`self.XsDotManager`)))
  (add `XsDot.OnButtonClicked` _xsdot (delegate `커스텀이벤트`))
  (`XsDot.AddBindingManager` _xsdot (`self.XsBindingManager`))
  (for (_array_element _array_index) (`self.BindingTagAndDeviceAddress`)
    (`XsBindingManager.Bind` (`self.XsBindingManager`) "" (make `XsBindingInfo` (`|GetArrayItem` (`|MakeArray` (`self.Rotation1`) (`self.Rotation2`) (`self.Rotation3`)) _array_index) (`.DeviceBluetoothAddress_5_044B8B224C3249DC1F00198B6CAF3C2E` (break `/Game/Assets/Blueprints/Struct/BindingMinimalInfo` _array_element)) true true) true)))

(event `커스텀이벤트`
  (params (deviceAddress :type String) (timestamp :type Integer)))

(event `self.ControlRig.OnPreInitializeDelegate`
  (params (Component :type "ControlRigComponent Object Reference"))
  (`ControlRigComponent.AddMappedCompleteSkeletalMesh` Component (`self.Mesh`)))

(event `self.ControlRig.OnPreForwardsSolveDelegate`
  (params (Component :type "ControlRigComponent Object Reference"))
  (bind _ascr_xs_binded (cast `/Game/Assets/Mesh/CR_XsBinded` (`ControlRigComponent.GetControlRig` Component)))
  (set `/Game/Assets/Mesh/CR_XsBinded.ShoulderRotation` (`KismetMathLibrary.Conv_RotatorToQuaternion` (`SceneComponent.RelativeRotation` (`self.Rotation1`))) _ascr_xs_binded)
  (set `/Game/Assets/Mesh/CR_XsBinded.ForeArmRotation` (`KismetMathLibrary.Conv_RotatorToQuaternion` (`SceneComponent.RelativeRotation` (`self.Rotation2`))) _ascr_xs_binded)
  (set `/Game/Assets/Mesh/CR_XsBinded.HandRotation` (`KismetMathLibrary.Conv_RotatorToQuaternion` (`SceneComponent.RelativeRotation` (`self.Rotation3`))) _ascr_xs_binded))

(fn `UserConstructionScript`)