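; BP_Polyman is a character Blueprint whose mesh is driven by a Control Rig component, set up for a look-at behavior.
; BeginPlay defaults LookingTarget to the player pawn if unset, and rig pre-initialization maps the complete skeletal mesh to the rig.
; Logic to pass the target location and IsLooking flag to CR_People exists but is disconnected, leaving the pre-forwards-solve event empty.
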(event `self.ReceiveBeginPlay`
  (`/Engine/EditorBlueprintResources/StandardMacros.IsValid` (`self.LookingTarget`)
    (:`Is Not Valid`
      (set `self.LookingTarget` (`GameplayStatics.GetPlayerPawn` 0)))))

(event `self.ControlRig.OnPreInitializeDelegate`
  (params (Component :type "ControlRigComponent Object Reference"))
  (`ControlRigComponent.AddMappedCompleteSkeletalMesh` Component (`self.Mesh`)))

(event `self.ControlRig.OnPreForwardsSolveDelegate`
  (params (Component :type "ControlRigComponent Object Reference")))

(fn `UserConstructionScript`)