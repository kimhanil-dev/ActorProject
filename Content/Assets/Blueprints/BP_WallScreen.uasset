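; BP_WallScreen is a wall screen actor whose displayed image can be changed and faded out at runtime.
; On BeginPlay it creates a dynamic instance of MT_ScreenWall on its static mesh.
; ChangeTexture looks up a name in the Textures map and, if found, sets the MainTexture parameter.
; PlayFadeOut sets FadeOutAlpha to full at once; a delayed reset to zero exists but is disconnected.
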(event `self.ReceiveBeginPlay`
  (bind _returnvalue (`PrimitiveComponent.CreateDynamicMaterialInstance` (`self.StaticMesh`) 0 "/Game/Assets/Materials/MT_ScreenWall.MT_ScreenWall" "None"))
  (set `self.ScreenWallMaterial` _returnvalue))

(event `ChangeTexture`
  (params (TextureName :type String))
  (bind (_value _returnvalue) (`BlueprintMapLibrary.Map_Find` (`self.Textures`) TextureName))
  (if _returnvalue
    (`MaterialInstanceDynamic.SetTextureParameterValue` (`self.ScreenWallMaterial`) "MainTexture" _value)))

(event `PlayFadeOut`
  (`MaterialInstanceDynamic.SetScalarParameterValue` (`self.ScreenWallMaterial`) "FadeOutAlpha" 1.0))

(fn `UserConstructionScript`)