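; BP_Bones is an actor that rotates a set of three joints to follow the entries in its XsSenserBinders array.
; BeginPlay collects Joint0, Joint1 and Joint2 into the Joints array.
; Each Tick pairs binders to joints by index and copies the world rotation of each binder's own Joint0 into the matching joint's relative rotation, with no space conversion or bounds check.
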(event `self.ReceiveBeginPlay`
  (`KismetArrayLibrary.Array_Add` (`self.Joints`) (`self.Joint0`))
  (`KismetArrayLibrary.Array_Add` (`self.Joints`) (`self.Joint1`))
  (`KismetArrayLibrary.Array_Add` (`self.Joints`) (`self.Joint2`)))

(event `self.ReceiveTick`
  (params (DeltaSeconds :type "Float (single-precision)"))
  (for (_array_element _array_index) (`self.XsSenserBinders`)
    (`SceneComponent.K2_SetRelativeRotation` (`|GetArrayItem` (`self.Joints`) _array_index) (`SceneComponent.K2_GetComponentRotation` (`/Game/Assets/Blueprints/BP_XsDotTester.Joint0` _array_element)) false false)))

(fn `UserConstructionScript`)