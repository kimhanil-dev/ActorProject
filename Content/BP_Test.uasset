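; BP_Test is a test actor that drives a Cube component from live XsDot Bluetooth motion sensor data.
; On BeginPlay it scans for ten seconds, stores the detected device addresses, then connects the devices after a short delay.
; Each Tick reads the first device's live data and, when valid, sets the cube's world rotation from it and adds raw acceleration as an unswept world offset, unscaled by delta time.
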(event `self.ReceiveBeginPlay`
  (bind _xsdot (`self.XsDot`))
  (`XsDot.StartScanning` _xsdot)
  (`KismetSystemLibrary.Delay` 10.0)
  (`XsDot.StopScanning` _xsdot)
  (bind _devices (`XsDot.GetDetectedDeviceName` _xsdot))
  (for _array_element _devices
    (`KismetArrayLibrary.Array_Add` (`self.DeviceBluetoothAddresses`) (`.BluetoothAddress` (break `XsPortInfo` _array_element))))
  (`KismetSystemLibrary.Delay` 1.0)
  (`XsDot.ConnectDevices` _xsdot))

(event `self.ReceiveTick`
  (params (DeltaSeconds :type "Float (single-precision)"))
  (bind _devicebluetoothaddresses (`self.DeviceBluetoothAddresses`))
  (bind _cube (`self.Cube`))
  (if (not (`KismetArrayLibrary.Array_IsEmpty` _devicebluetoothaddresses))
    (bind (_rotation _acceleration _valid) (`XsDot.GetLiveData` (`self.XsDot`) (`|GetArrayItem` _devicebluetoothaddresses)))
    (if _valid
      (`SceneComponent.K2_SetWorldRotation` _cube (`KismetMathLibrary.MakeRotator` (.x _rotation) (.y _rotation) (.z _rotation)) false false)
      (`SceneComponent.K2_AddWorldOffset` _cube _acceleration false false))))

(fn `UserConstructionScript`)